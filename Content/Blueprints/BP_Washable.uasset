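; Washable actor whose static mesh carries a render-target dirt layer that can be cleaned at given UV positions.
; BeginPlay creates dirt alpha and albedo targets, bakes the albedo once from a generator material, and feeds both into the mesh's dynamic washing material.
; CleanTextureAtUV draws a brush material, which samples the alpha target, back into that target at the hit UV.
; An initial off-UV stroke runs at startup.
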(event EventBeginPlay
  (bind _dirttexturesize (Variables|Default|GetDirtTextureSize))
  (bind _dirttexturesize_2 (Variables|Default|GetDirtTextureSize))
  (Utilities|FlowControl|Sequence
    (:then_0
      (bind _returnvalue (Rendering|CreateRenderTarget2D _dirttexturesize_2 _dirttexturesize_2 "RTF_RGBA16f" "(R=1.000000,G=1.000000,B=1.000000,A=1.000000)"))
      (Variables|Default|SetDirtAlphaRenderTarget _returnvalue)
      (bind _returnvalue_2 (Rendering|CreateRenderTarget2D _dirttexturesize _dirttexturesize "RTF_RGBA16f" "(R=1.000000,G=0.000000,B=1.000000,A=1.000000)"))
      (Variables|Default|SetDirtAlbedoRenderTarget _returnvalue_2))
    (:then_1
      (bind _returnvalue_3 (Rendering|Material|CreateDynamicMaterialInstance (Variables|Default|GetStaticMesh) 0 "/Game/Materials/BrushMaterial.BrushMaterial" "None" :!class /Script/Engine.PrimitiveComponent))
      (Variables|Default|SetBrushStrokeMat _returnvalue_3)
      (Rendering|Material|SetTextureParameterValue (Variables|Default|GetBrushStrokeMat) "DirtTexture" (Variables|Default|GetDirtAlphaRenderTarget))
      (CallFunction|CleanTextureatUV "(X=100000.000000,Y=100000.000000)" 0.0))
    (:then_2
      (bind _returnvalue_4 (Rendering|Material|CreateDynamicMaterialInstance (Variables|Default|GetStaticMesh) 0 "/Game/Materials/DirtTextureGenerator.DirtTextureGenerator" "None" :!class /Script/Engine.PrimitiveComponent))
      (Variables|Default|SetDirtTextureGenerator _returnvalue_4)
      (Rendering|DrawMaterialtoRenderTarget (Variables|Default|GetDirtAlbedoRenderTarget) (Variables|Default|GetDirtTextureGenerator)))
    (:then_3
      (bind _returnvalue_5 (Rendering|Material|CreateDynamicMaterialInstance (Variables|Default|GetStaticMesh) 0 "/Game/Materials/WashingMaterial.WashingMaterial" "None" :!class /Script/Engine.PrimitiveComponent))
      (Variables|Default|SetRenderMaterial _returnvalue_5)
      (Rendering|Material|SetTextureParameterValue (Variables|Default|GetRenderMaterial) "DirtTexture" (Variables|Default|GetDirtAlphaRenderTarget))
      (Rendering|Material|SetTextureParameterValue (Variables|Default|GetRenderMaterial) "DirtAlbedo" (Variables|Default|GetDirtAlbedoRenderTarget))
      (Rendering|Material|SetMaterial (Variables|Default|GetStaticMesh) 0 (Variables|Default|GetRenderMaterial)))))

(fn ConstructionScript)

(fn CleanTextureatUV
  (params (In%20UV :type Vector%202D%20Structure) (UVToWorldRatio :type Float%20%28double-precision%29))
  (bind (_x _y) (Math|Vector2D|BreakVector2D In%20UV))
  (Rendering|Material|SetVectorParameterValue (Variables|Default|GetBrushStrokeMat) "HitPos" (Utilities|Struct|MakeLinearColor _x _y 0.0 1.0) :!class /Script/Engine.MaterialInstanceDynamic)
  (Rendering|Material|SetScalarParameterValue (Variables|Default|GetBrushStrokeMat) "UVToWorldRatio" UVToWorldRatio :!class /Script/Engine.MaterialInstanceDynamic)
  (Rendering|DrawMaterialtoRenderTarget (Variables|Default|GetDirtAlphaRenderTarget) (Variables|Default|GetBrushStrokeMat)))